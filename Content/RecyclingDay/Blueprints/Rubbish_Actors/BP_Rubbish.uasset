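; BP_Rubbish is a destructible rubbish sprite actor that reacts to ball impacts and is destroyed on the fourth hit.
; The BIBallImpact event increments HitCount and branches on the new value.
; The first three hits tint the sprite progressively darker and play an impact sound, with the first also clearing the overlay material.
; The final hit destroys the actor and plays a wood impact sound.
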(event `/Game/RecyclingDay/Blueprints/BI_Ball.BI Ball Impact`
  (bind _rubbish (`self.Rubbish`))
  (bind _result (`/Engine/EditorBlueprintResources/StandardMacros.IncrementInt` (`self.HitCount`))
    (:`  `
      (if (== _result 1)
        (`PaperSpriteComponent.SetSpriteColor` _rubbish (struct :`R` 0.8 :`G` 0.673068 :`B` 0.06695 :`A` 1.0))
        (`MeshComponent.SetOverlayMaterial` _rubbish null)
        (`GameplayStatics.PlaySound2D` "/Game/Sounds/impact_stone_1.impact_stone_1" 1.0 1.0 0.0 null null)
        (elif (== _result 2)
          (`PaperSpriteComponent.SetSpriteColor` _rubbish (struct :`R` 0.6 :`G` 0.219164 :`B` 0.036632 :`A` 1.0))
          (`GameplayStatics.PlaySound2D` "/Game/Sounds/impact_stone_2.impact_stone_2" 1.0 1.0 0.0 null null)
          (elif (== _result 3)
            (`PaperSpriteComponent.SetSpriteColor` _rubbish (struct :`R` 0.4 :`G` 0.013038 :`A` 1.0))
            (`GameplayStatics.PlaySound2D` "/Game/Sounds/impact_metal_1.impact_metal_1" 1.0 1.0 0.0 null null)
            (elif (== _result 4)
              (`self.K2_DestroyActor`)
              (`GameplayStatics.PlaySound2D` "/Game/Sounds/impact_wood_1.impact_wood_1" 1.0 1.0 0.0 null null))))))))

(fn `UserConstructionScript`)