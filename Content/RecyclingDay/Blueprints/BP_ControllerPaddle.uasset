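; BP_ControllerPaddle is the controller for the paddle in RecyclingDay, turning mouse movement into paddle motion.
; On possess it caches the pawn as a BP_Paddle.
; The Move Mouse axis, scaled by sensitivity, selects move right, move left or stop by its sign.
; While moving, the scaled rate also feeds the paddle's timeline play rate, so mouse speed drives paddle speed.
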(event `self.ReceivePossess`
  (params (PossessedPawn :type "Pawn Object Reference"))
  (bind _asbp_paddle (cast `/Game/RecyclingDay/Blueprints/BP_Paddle` PossessedPawn))
  (set `self.As BP Paddle` _asbp_paddle))

(event `InputAxis|Move Mouse`
  (params (AxisValue :type "Float (single-precision)"))
  (bind _as_bp_paddle (`self.As BP Paddle`))
  (bind _mouse_move_rate (`self.Mouse Move Rate`))
  ;[0.1 1 0.5] Move Bat
  (bind _output_get (set `self.Mouse Move Rate` (* AxisValue (`self.Mouse Sensitivity`))))
  (`/Engine/EditorBlueprintResources/StandardMacros.CompareFloat` _output_get
    (:`>`
      (`/Game/RecyclingDay/Blueprints/BP_Paddle.Move Right` _as_bp_paddle)
      (`/Game/RecyclingDay/Blueprints/BP_Paddle.Update Timeline Play Rate` _as_bp_paddle _mouse_move_rate :!label _label))
    (:`==`
      (`/Game/RecyclingDay/Blueprints/BP_Paddle.Stop Moving` _as_bp_paddle))
    (:`<`
      (`/Game/RecyclingDay/Blueprints/BP_Paddle.Move Left` _as_bp_paddle)
      (`/Engine/EditorBlueprintResources/StandardMacros.NegateFloat` _mouse_move_rate
        (:`  `
          (goto _label))))))

(fn `UserConstructionScript`)