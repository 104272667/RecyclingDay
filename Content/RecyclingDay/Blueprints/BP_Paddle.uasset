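; Player bat for the Recycling Day game that slides left and right along a spline.
; A Timeline drives the motion: MoveRight plays it, MoveLeft reverses it, and its track value scales spline length to position PaddleAnchor.
; The spline transform is sampled in local space but applied as a world transform.
; Other events stop the Timeline, reset its time (also on BeginPlay) and change its play rate.
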(event `self.ReceiveBeginPlay`
  ;[1 1 1] Setup
  (`self.Reset Bat`))

(event `Move Right`
  (bind _spline (`self.Spline`))
  ;[0 0.8189 1] Move Bat
  (bind (_direction _newtrack_0) (`Timeline|Timeline` :!label _label)
    (:`Update`
      (`SceneComponent.K2_SetWorldTransform` (`self.PaddleAnchor`) (`SplineComponent.GetTransformAtDistanceAlongSpline` _spline (* (`SplineComponent.GetSplineLength` _spline) _newtrack_0) "Local" false) false false))))

(event `Stop Moving`
  ;[0 0.8189 1] Move Bat
  (goto _label :!via `Stop`))

(event `Move Left`
  ;[0 0.8189 1] Move Bat
  (goto _label :!via `Reverse`))

(event `Reset Bat`
  ;[0 0.8189 1] Move Bat
  (goto _label :!via `SetNewTime`))

(event `Update Timeline Play Rate`
  (params (NewRate :type "Float (single-precision)"))
  (`TimelineComponent.SetPlayRate` (`self.Timeline`) NewRate))

(fn `UserConstructionScript`)